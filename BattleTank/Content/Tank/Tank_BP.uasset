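; Player-controlled tank pawn Blueprint that assembles its meshes and routes input to aiming, driving and firing.
; BeginPlay assigns track, turret and barrel meshes, then passes the barrel and turret references to the tank through setter calls.
; Aim axes rotate an azimuth gimbal and spring arm separately from the turret.
; Left and right throttle axes drive each track independently, and the fire action calls Fire.
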(event `self.ReceiveBeginPlay`
  (`StaticMeshComponent.SetStaticMesh` (`self.RightTrack`) "/Game/Tank/tank_fbx_Track.tank_fbx_Track")
  (`StaticMeshComponent.SetStaticMesh` (`self.LeftTrack`) "/Game/Tank/tank_fbx_Track.tank_fbx_Track")
  (`StaticMeshComponent.SetStaticMesh` (`self.Turret`) "/Game/Tank/tank_fbx_Turret.tank_fbx_Turret")
  (`StaticMeshComponent.SetStaticMesh` (`self.Barrel`) "/Game/Tank/tank_fbx_Barrel.tank_fbx_Barrel")
  (`self.SetBarrelReference` (`self.Barrel`))
  (`self.SetTurretReference` (`self.Turret`)))

(event `InputAxis|AimAzimuth`
  (params (AxisValue :type "Float (single-precision)"))
  ;[1 1 1] Input Binding
  (`SceneComponent.K2_AddLocalRotation` (`self.Azimuth Gimbal`) (`KismetMathLibrary.MakeRotator` 0.0 0.0 AxisValue) false false))

(event `InputAxis|AimElevation`
  (params (AxisValue :type "Float (single-precision)"))
  ;[1 1 1] Input Binding
  (`SceneComponent.K2_AddLocalRotation` (`self.SpringArm`) (`KismetMathLibrary.MakeRotator` 0.0 AxisValue) false false))

(event `InputAction|fire`
  (params (Key :type "Key Structure"))
  ;[1 1 1] Input Binding
  (:`Pressed`
    (`self.Fire`)))

(event `InputAxis|LeftThrottle`
  (params (AxisValue :type "Float (single-precision)"))
  ;[1 1 1] Input Binding
  (`TankTrack.SetThrottle` (`self.LeftTrack`) AxisValue))

(event `InputAxis|RightThrottle`
  (params (AxisValue :type "Float (single-precision)"))
  ;[1 1 1] Input Binding
  (`TankTrack.SetThrottle` (`self.RightTrack`) AxisValue))

(fn `UserConstructionScript`)